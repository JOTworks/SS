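; Checkpoint actor that records itself as the saved checkpoint when any actor overlaps it.
; On overlap it takes the slot name from SSGameMode, loads the existing SSSaveGame, stores its own display name as Checkpoint and saves back to the slot.
; It prints the saved name, or a shared failure message if either cast fails, and does not create a save.
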(event `self.ReceiveActorBeginOverlap`
  (params (OtherActor :type "Actor Object Reference"))
  (bind _asssgame_mode (cast `/Game/Blueprints/SSGameMode` (`GameplayStatics.GetGameMode`))
    (:`then`
      (bind _slot_name (`/Game/Blueprints/SSGameMode.Slot Name` _asssgame_mode))
      (bind _returnvalue (`GameplayStatics.LoadGameFromSlot` _slot_name))
      (bind _assssave_game (cast `/Game/Blueprints/SSSaveGame` _returnvalue)
        (:`then`
          (bind _output_get (set `/Game/Blueprints/SSSaveGame.Checkpoint` (`KismetSystemLibrary.GetDisplayName` self) _assssave_game))
          (`GameplayStatics.SaveGameToSlot` _assssave_game _slot_name)
          (`KismetSystemLibrary.PrintString` _output_get))
        (:`CastFailed`
          (`KismetSystemLibrary.PrintString` "checkpoint: cast to SSgamemode failed" :!label _label))))
    (:`CastFailed`
      (goto _label))))

(fn `UserConstructionScript`)