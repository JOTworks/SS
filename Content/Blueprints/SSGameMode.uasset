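; Side-scroller game mode that handles startup, the main menu and the transition into play.
; BeginPlay writes a default save, moves the player to the Checkpoint actor whose display name matches the saved one, switches to the start camera and adds both menus.
; The play button event hides the main menu, blends back to the player camera and sets IsReadyAnimation.
; The default checkpoint also calls PlayOpeningSequence, which is an empty stub.
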(event `self.ReceiveBeginPlay`
  (`|ExecutionSequence`
    (:`then_0`
      (bind _asside_scroller_character (cast `/Game/SideScrollerBP/Blueprints/SideScrollerCharacter` (`GameplayStatics.GetPlayerPawn` 0))
        (:`then`
          (`/Game/SideScrollerBP/Blueprints/SideScrollerCharacter.deactivateZoomCam` _asside_scroller_character)
          (set `self.playerCamera` (`Controller.GetViewTarget` (`GameplayStatics.GetPlayerController` 0)))
          (`/Game/SideScrollerBP/Blueprints/SideScrollerCharacter.setup for superzoom` _asside_scroller_character))
        (:`CastFailed`
          (`KismetSystemLibrary.PrintString` "SSGameMode: cast to sidescrfollercharacter failed"))))
    (:`then_1`
      ;[1 1 1] if there is no save game, creates one with the starting position as the checkpoint
      (bind _returnvalue (`GameplayStatics.DoesSaveGameExist` (`self.Slot Name`)))
      (if _returnvalue
        _
        (else
          _))
      (`|ExecutionSequence`
        (:`then_0`
          (bind _returnvalue_2 (`GameplayStatics.CreateSaveGameObject` "/Game/Blueprints/SSSaveGame.SSSaveGame_C"))
          (set `/Game/Blueprints/SSSaveGame.Checkpoint` "checkpoint" _returnvalue_2)
          (set `/Game/Blueprints/SSSaveGame.sound` true _returnvalue_2)
          (set `/Game/Blueprints/SSSaveGame.music` true _returnvalue_2)
          (`GameplayStatics.SaveGameToSlot` _returnvalue_2 (`self.Slot Name`)))))
    (:`then_2`
      ;[1 1 1] moves character to starting checkpoint
      (bind _outactors (`GameplayStatics.GetAllActorsOfClass` "/Game/Blueprints/checkpoint.checkpoint_C"))
      (bind _returnvalue_3 (`GameplayStatics.LoadGameFromSlot` (`self.Slot Name`)))
      (bind _assssave_game (cast `/Game/Blueprints/SSSaveGame` _returnvalue_3)
        (:`then`
          (set `self.startingCheckPoint` (`/Game/Blueprints/SSSaveGame.Checkpoint` _assssave_game))
          (for _array_element _outactors
            (bind _returnvalue_4 (`KismetSystemLibrary.GetDisplayName` _array_element))
            (if (`KismetStringLibrary.EqualEqual_StrStr` _returnvalue_4 (`self.startingCheckPoint`))
              (`KismetSystemLibrary.PrintString` _returnvalue_4)
              (`self.K2_SetActorLocation` (`GameplayStatics.GetPlayerPawn` 0) (`self.K2_GetActorLocation` _array_element) false false)
              (break)
              (else
                (`KismetSystemLibrary.PrintString` "false")))))
        (:`CastFailed`
          (`KismetSystemLibrary.PrintString` "SSgamemode: cast to sssavegame failed"))))
    (:`then_3`
      (bind _outactors_2 (`GameplayStatics.GetAllActorsOfClass` "/Game/Blueprints/Start_camera.Start_camera_C"))
      (`PlayerController.SetViewTargetWithBlend` (`GameplayStatics.GetPlayerController` 0) (`|GetArrayItem` _outactors_2) 0.0 "VTBlend_Linear" 0.0 false)
      (bind _returnvalue_5 (`|CreateWidget` "/Game/UI/Main_Menu.Main_Menu_C"))
      (bind _output_get (set `self.mainMenu` _returnvalue_5))
      (`UserWidget.AddToViewport` _output_get 0)
      (bind _returnvalue_6 (`|CreateWidget` "/Game/UI/pause_menu.pause_menu_C"))
      (`UserWidget.AddToViewport` _returnvalue_6 0))))

(event `play game button`
  (`Widget.SetVisibility` (`self.mainMenu`) "Hidden")
  (`KismetSystemLibrary.Delay` 0.5)
  (bind _returnvalue (`GameplayStatics.LoadGameFromSlot` (`self.Slot Name`)))
  (bind _assssave_game (cast `/Game/Blueprints/SSSaveGame` _returnvalue)
    (:`then`
      (if (`KismetStringLibrary.EqualEqual_StrStr` (`/Game/Blueprints/SSSaveGame.Checkpoint` _assssave_game) "checkpoint")
        (`PlayerController.SetViewTargetWithBlend` (`GameplayStatics.GetPlayerController` 0) (`self.playerCamera`) 1.0 "VTBlend_Cubic" 0.0 false)
        (`self.playOpeningSequence`)
        (else
          (`PlayerController.SetViewTargetWithBlend` (`GameplayStatics.GetPlayerController` 0) (`self.playerCamera`) 1.0 "VTBlend_Cubic" 0.0 false)))
      (`KismetSystemLibrary.Delay` 1.0)
      (set `self.isReadyAnimation` true))
    (:`CastFailed`
      (`KismetSystemLibrary.PrintString` "SSgamemode: cast to sssavegame failed"))))

(fn `playOpeningSequence`)

(fn `UserConstructionScript`)